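; Main menu actor that creates and switches the front-end menu screens and their background music.
; It polls every 0.1 seconds until the Game Instance's launch check passes, then creates the widgets and sounds, binds to StateChanged and sets the main menu state.
; Each state change hides the old screen, shows the new one and fades menu or options music.
; The Audio Options state shows the Instructions widget, and controls music is never played.
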(event `self.ReceiveBeginPlay`
  (bind _asbp_game_instance (cast `/Game/TopDownStealthToolkit/Blueprints/BP_GameInstance` (`GameplayStatics.GetGameInstance`)))
  (set `self.GameInstanceRef` _asbp_game_instance)
  (`self.Initialize`))

(event `Initialize`
  (bind _returnvalue (`GameplayStatics.GetPlayerController` 0))
  ;[1 1 1] Custom event used to load the main menu, once all the pre requisites are executed by the Game Instance class
  (if (`/Game/TopDownStealthToolkit/Blueprints/BP_GameInstance.GameLaunchEventCheck` (`self.GameInstanceRef`)) :!label _label
    ;[1 1 1] Create Main Menu Widget and Bind to StateChanged Event of Game Instance
    (`|ExecutionSequence`
      (:`then_0`
        (bind _returnvalue_2 (`|CreateWidget` "/Game/UI/Widgets/Widget_MainMenu.Widget_MainMenu_C" _returnvalue))
        (set `self.MainMenu` _returnvalue_2)
        (bind _returnvalue_3 (`GameplayStatics.CreateSound2D` "/Game/Audio/MainMenuSFX/mainMenuBGM.mainMenuBGM"))
        (set `self.MenuBGM` _returnvalue_3))
      (:`then_1`
        (bind _returnvalue_4 (`|CreateWidget` "/Game/UI/Widgets/WidgetBP_OptionsMenuScreen.WidgetBP_OptionsMenuScreen_C" _returnvalue))
        (set `self.OptionsMenu` _returnvalue_4)
        (bind _returnvalue_5 (`GameplayStatics.CreateSound2D` "/Game/Audio/MenuBGM/OptionsMenuBGM.OptionsMenuBGM"))
        (set `self.OptionsBGM` _returnvalue_5))
      (:`then_2`
        (bind _returnvalue_6 (`|CreateWidget` "/Game/UI/Widgets/WidgetBP_VideoOptionScreen.WidgetBP_VideoOptionScreen_C" _returnvalue))
        (set `self.VideoOptionsMenu` _returnvalue_6))
      (:`then_3`
        (bind _returnvalue_7 (`|CreateWidget` "/Game/UI/Widgets/WidgetBP_GameplayOptionsScreen.WidgetBP_GameplayOptionsScreen_C" _returnvalue))
        (set `self.GameplayOptionsMenu` _returnvalue_7))
      (:`then_4`
        (bind _returnvalue_8 (`|CreateWidget` "/Game/UI/Widgets/WidgetBP_ControlsScreen.WidgetBP_ControlsScreen_C"))
        (set `self.ControlsMenu` _returnvalue_8)
        (bind _returnvalue_9 (`GameplayStatics.CreateSound2D` "/Game/Audio/MenuBGM/ControlMenuBGM.ControlMenuBGM"))
        (set `self.ControlsBGM` _returnvalue_9))
      (:`then_5`
        (bind _returnvalue_10 (`|CreateWidget` "/Game/UI/Widgets/WidgetBP_InstructionsScreen.WidgetBP_InstructionsScreen_C"))
        (set `self.InstructionsMenu` _returnvalue_10))
      (:`then_6`
        (add `/Game/TopDownStealthToolkit/Blueprints/BP_GameInstance.StateChanged` (`self.GameInstanceRef`) (delegate `OnStateChanged`)))
      (:`then_7`
        ;[1 1 1] Set State of Game Instance to Main Menu State
        (`/Game/TopDownStealthToolkit/Blueprints/BP_GameInstance.SetGameState` (`self.GameInstanceRef`) "NewEnumerator0")))
    (else
      (`KismetSystemLibrary.Delay` 0.1)
      (goto _label))))

(event `OnStateChanged`
  (params (OldState :type "/Game/Blueprints/Enums/EGameState Enum") (NewState :type "/Game/Blueprints/Enums/EGameState Enum"))
  (bind _menubgm (`self.MenuBGM`))
  (bind _optionsbgm (`self.OptionsBGM`))
  (bind _mainmenu (`self.MainMenu`))
  ;[1 1 1] Handle state change event notification from game instance
  (`|ExecutionSequence`
    (:`then_0`
      (switch `/Game/Blueprints/Enums/EGameState` OldState
        (:`NewEnumerator0`
          (`Widget.SetVisibility` (`self.MainMenu`) "Collapsed")
          (if (not (`|EnumEquality` "NewEnumerator15" NewState))
            (`AudioComponent.FadeOut` (`self.MenuBGM`) 1.0 0.0)
            (`KismetSystemLibrary.Delay` 1.75)))
        (:`NewEnumerator2`
          (`Widget.RemoveFromParent` (`self.OptionsMenu`))
          (if (`|EnumEquality` NewState "NewEnumerator0")
            (`AudioComponent.FadeOut` (`self.OptionsBGM`) 1.0 0.0)
            (`KismetSystemLibrary.Delay` 1.0)))
        (:`NewEnumerator7`
          (`Widget.RemoveFromParent` (`self.VideoOptionsMenu`)))
        (:`NewEnumerator13`
          (`Widget.RemoveFromParent` (`self.GameplayOptionsMenu`)))
        (:`NewEnumerator14`
          (`Widget.RemoveFromParent` (`self.InstructionsMenu`)))
        (:`NewEnumerator15`
          (`Widget.RemoveFromParent` (`self.ControlsMenu`)))))
    (:`then_1`
      (switch `/Game/Blueprints/Enums/EGameState` NewState
        (:`NewEnumerator0`
          (`|ExecutionSequence`
            (:`then_0`
              (`/Engine/EditorBlueprintResources/StandardMacros.DoOnce` false
                (:`Completed`
                  (`UserWidget.AddToViewport` _mainmenu 0))))
            (:`then_1`
              (`Widget.SetVisibility` _mainmenu "Visible")))
          (set `PlayerController.bShowMouseCursor` true (`GameplayStatics.GetPlayerController` 0))
          (`/Engine/EditorBlueprintResources/StandardMacros.IsValid` _menubgm
            (:`Is Valid`
              (if (not (`|EnumEquality` OldState "NewEnumerator15"))
                (`AudioComponent.FadeIn` _menubgm 0.4 1.0 0.0)))
            (:`Is Not Valid`
              (bind _returnvalue (`GameplayStatics.CreateSound2D` "/Game/Audio/MainMenuSFX/mainMenuBGM.mainMenuBGM"))
              (bind _output_get (set `self.MenuBGM` _returnvalue))
              (`AudioComponent.FadeIn` _output_get 0.5 1.0 0.0))))
        (:`NewEnumerator2`
          (`UserWidget.AddToViewport` (`self.OptionsMenu`) 0)
          (set `PlayerController.bShowMouseCursor` true (`GameplayStatics.GetPlayerController` 0))
          (`/Engine/EditorBlueprintResources/StandardMacros.IsValid` _optionsbgm
            (:`Is Valid`
              (`/Engine/EditorBlueprintResources/StandardMacros.DoOnce` false
                (:`Completed`
                  (`AudioComponent.FadeIn` _optionsbgm 0.5 1.0 0.0))))
            (:`Is Not Valid`
              (if (not (`|EnumEquality` OldState "NewEnumerator2"))
                (bind _returnvalue_2 (`GameplayStatics.CreateSound2D` "/Game/Audio/MenuBGM/OptionsMenuBGM.OptionsMenuBGM"))
                (bind _output_get_2 (set `self.OptionsBGM` _returnvalue_2))
                (`AudioComponent.FadeIn` _output_get_2 0.5 1.0 0.0)))))
        (:`NewEnumerator3`
          (`AudioComponent.FadeOut` (`self.MenuBGM`) 1.0 0.0)
          (`KismetSystemLibrary.Delay` 1.75))
        (:`NewEnumerator7`
          (`UserWidget.AddToViewport` (`self.VideoOptionsMenu`) 0)
          (set `PlayerController.bShowMouseCursor` true (`GameplayStatics.GetPlayerController` 0) :!label _label_2))
        (:`NewEnumerator13`
          (`UserWidget.AddToViewport` (`self.GameplayOptionsMenu`) 0)
          (goto _label_2))
        (:`NewEnumerator14`
          (`UserWidget.AddToViewport` (`self.InstructionsMenu`) 0)
          (goto _label_2))
        (:`NewEnumerator15`
          (`UserWidget.AddToViewport` (`self.ControlsMenu`) 0)
          (goto _label_2))))))

(event `self.ReceiveDestroyed`
  ;[1 1 1] Unbind State Change Event Handler if actor is destroyed
  (remove `/Game/TopDownStealthToolkit/Blueprints/BP_GameInstance.StateChanged` (`self.GameInstanceRef`) (delegate `OnStateChanged`)))

(fn `UserConstructionScript`)